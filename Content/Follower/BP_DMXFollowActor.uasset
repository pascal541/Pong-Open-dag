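; Pong-style ball actor that moving-head DMX fixtures track as it bounces around a two-player field.
; Tick moves the ball, speeds it up on bounces, checks paddle misses, mirrors scores over DMX and polls DMX input for reset and start.
; On movement, throttled by a refresh timer, it aims tagged helper components on each selected BP_Mover at the ball, converting their rotations to pan/tilt DMX values scaled by range and bit depth.
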(event `self.ReceiveBeginPlay`
  (set `self.velocity_Backup` (`self.velocity`))
  (set `self.PrevLocation` (`self.K2_GetActorLocation`))
  (`DMXSubsystem.SendDMXToOutputPort` (struct :`PortGuid` "2B8E1B6D4FCE28BABE657BA340F90118" :`bEnabledFlag` true) (`|MakeMap` 100 :!valuetype "Byte") 2)
  ;[1 0 0] Update Ball in DMX
  (`self.UpdateSelectedPatches` :!label _label)
  (`KismetSystemLibrary.K2_SetTimerDelegate` (delegate `ReadyToUpdate`) (`self.RefreshRateInSeconds`)))

(event `self.ReceiveTick`
  (params (DeltaSeconds :type "Float (single-precision)"))
  (bind _radius (`self.Radius`))
  (bind (_fieldsize_x _fieldsize_y) (`KismetMathLibrary.BreakVector` (`self.FieldSize`)))
  (bind _score (`self.Score`))
  (bind _maxscore (`self.MaxScore`))
  (bind (_velocity_x _velocity_y _velocity_z) (`KismetMathLibrary.BreakVector` (`self.velocity`)))
  (bind (_velocity_x_2 _velocity_y_2 _velocity_z_2) (`KismetMathLibrary.BreakVector` (`self.velocity`)))
  (bind _x (.x (`self.K2_GetActorLocation`)))
  (bind _y (.y (`self.K2_GetActorLocation`)))
  (bind _returnvalue (< _y (+ (* -1 _fieldsize_y) _radius)))
  ;[1 1 1] Timing System
  (`|ExecutionSequence`
    (:`then_0`
      (if (and (!= (`self.PrevLocation`) (`self.K2_GetActorLocation`)) (`self.CanUpdate`))
        (set `self.CanUpdate` false)
        (goto _label)))
    (:`then_1`
      (if (`self.Playing`)
        ;[0 1 0] Move Ball in Unreal
        (set `self.PrevLocation` (`self.K2_GetActorLocation`))
        (`self.K2_AddActorWorldOffset` (`self.velocity`) true true)
        (`|ExecutionSequence`
          (:`then_0`
            ;[0 0 1] Bounce Up/Down
            (if (or (< _x (+ (* -1 _fieldsize_x) _radius)) (> _x (- _fieldsize_x _radius)))
              (set `self.velocity` (`KismetMathLibrary.MakeVector` (* -1 _velocity_x) _velocity_y _velocity_z))
              (`self.OnBounce`)))
          (:`then_1`
            (set `self.IsRight` _returnvalue)
            (if (or _returnvalue (> _y (- _fieldsize_y _radius)))
              (if (`self.Calibrating`)
                ;[0 0 1] Bounce Left/Right
                (set `self.velocity` (`KismetMathLibrary.MakeVector` _velocity_x_2 (* -1 _velocity_y_2) _velocity_z_2) :!label _label_2)
                (`self.OnBounce`)
                (else
                  ;[0 0 1] Check Goal
                  (`self.CheckGoal` _returnvalue
                    (:`True`
                      (`self.OnGoal`
                        (:`Óut`
                          ;[0 1 0] Update Score Counter in Unreal
                          (if (`self.IsRight`)
                            (set `self.Score` (+ _score (1.0 0.0 0.0)))
                            (bind _result (`/Engine/EditorBlueprintResources/StandardMacros.IncrementInt` (`/Game/Blueprints/BP_Player1.Score` (`self.Player1`)))
                              (:`  `
                                (if (>= _result _maxscore)
                                  ;[0 0 1] Reset ball
                                  (`self.Reset` false :!label _label_3
                                    (:`Óut`
                                      (`|ExecutionSequence`
                                        (:`then_0`
                                          (`KismetSystemLibrary.Delay` (`self.ResetDelay`))
                                          (goto _label_5 :!via `Open`))
                                        (:`then_1`
                                          _))))
                                  (else
                                    (`self.Reset` true false :!label _label_4
                                      (:`Óut`
                                        _))))))
                            (else
                              (set `self.Score` (+ _score (0.0 1.0 0.0)))
                              (bind _result_2 (`/Engine/EditorBlueprintResources/StandardMacros.IncrementInt` (`/Game/Blueprints/BP_Player2.Score` (`self.Player2`)))
                                (:`  `
                                  (if (>= _result_2 _maxscore)
                                    (goto _label_3)
                                    (else
                                      (goto _label_4)))))))
                          ;[1 0 0] Update Score Counter in DMX
                          (for _index (range 1 513)
                            (`DMXSubsystem.SendDMXToOutputPort` (struct :`PortGuid` "2B8E1B6D4FCE28BABE657BA340F90118" :`bEnabledFlag` true) (`|MakeMap` _index :!valuetype "Byte") 4))
                          (`DMXSubsystem.SendDMXToOutputPort` (struct :`PortGuid` "2B8E1B6D4FCE28BABE657BA340F90118" :`bEnabledFlag` true) (`|MakeMap` (`/Game/Blueprints/BP_Player1.Score` (`self.Player1`)) 255 :!valuetype "Byte") 4)
                          (`DMXSubsystem.SendDMXToOutputPort` (struct :`PortGuid` "2B8E1B6D4FCE28BABE657BA340F90118" :`bEnabledFlag` true) (`|MakeMap` (+ (`/Game/Blueprints/BP_Player2.Score` (`self.Player2`)) 10) 255 :!valuetype "Byte") 4))))
                    (:`False`
                      (goto _label_2))))))))))
    (:`then_2`
      (bind _dmxdata (`DMXSubsystem.GetDMXDataFromInputPort` (struct :`PortGuid` "BA32F88C481FEBD32A83798451A0DFE1" :`bEnabledFlag` true) 2))
      (if (`KismetArrayLibrary.Array_IsValidIndex` _dmxdata)
        (`|ExecutionSequence`
          (:`then_0`
            (if (== (`|GetArrayItem` _dmxdata 101) 255)
              (`self.CustomEvent ResetBall`)))
          (:`then_1`
            (if (== (`|GetArrayItem` _dmxdata 100) 255)
              (`KismetSystemLibrary.Delay` 5.0)
              (set `self.Playing` true)
              (goto _label_5 :!via `Close`))))))
    (:`then_3`
      (`/Engine/EditorBlueprintResources/StandardMacros.Gate` true :!label _label_5
        (:`Exit`
          (`DMXSubsystem.SendDMXToOutputPort` (struct :`PortGuid` "2B8E1B6D4FCE28BABE657BA340F90118" :`bEnabledFlag` true) (`|MakeMap` 201 255 :!valuetype "Byte") 4))))))

(event `ReadyToUpdate`
  ;[1 0 0] Update Ball in DMX
  (set `self.CanUpdate` true))

(event `CustomEvent ResetBall`
  ;[1 1 1] Events
  (`self.Reset` false :!label _label_6))

(event `InputAction|ResetBall`
  (params (Key :type "Key Structure"))
  ;[1 1 1] Events
  (:`Pressed`
    (goto _label_6)))

(event `CustomEvent PauseBall`
  ;[1 1 1] Events
  (bind _isa (`/Engine/EditorBlueprintResources/StandardMacros.FlipFlop` :!label _label_7)
    (:`A`
      _)
    (:`B`
      _))
  (set `self.Playing` _isa))

(event `InputAction|PauseBall`
  (params (Key :type "Key Structure"))
  ;[1 1 1] Events
  (:`Pressed`
    (goto _label_7)))

(fn `GetAllFixturePatches`
  (params (CustomTag :type Name))
  (`KismetArrayLibrary.Array_Clear` (`self.FixturePatch`))
  (bind _outactors (`GameplayStatics.GetAllActorsWithTag` CustomTag))
  (set `self.FixturePatch` _outactors))

(fn `Update Tilt`
  (params (object :type "Object Object Reference"))
  (locals (LocalPatch :type "DMXEntityFixturePatch Object Reference") (TiltRange :type "Float (double-precision)" :default 0.0) (MovingHeadRef :type "Actor Object Reference") (RotationPoint :type "SceneComponent Object Reference") (TiltPoint :type "SceneComponent Object Reference"))
  (bind _returnvalue (`self.GetComponentsByTag` "/Script/Engine.SceneComponent" "HeadTilt"))
  (bind _tiltpoint (`local.TiltPoint`))
  (bind _movingheadref (`local.MovingHeadRef`))
  (bind _relativerotation_roll (`KismetMathLibrary.BreakRotator` (`SceneComponent.RelativeRotation` _tiltpoint)))
  (bind _output (`|GetArrayItem` (`self.GetComponentsByTag` _movingheadref "/Script/Engine.SceneComponent" "YokeRot")))
  (if (`self.bTilt`)
    (bind _asbp_mover (cast `/Game/DMX/BP_Mover` object))
    (set `local.MovingHeadRef` _asbp_mover)
    (bind (_dmxchannel_minvalue _dmxchannel_maxvalue) (break `DMXChannelData` (`DMXFixtureComponentSingle.DMXChannel` (`/Game/DMX/BP_Mover.Tilt_Component` _asbp_mover))))
    (set `local.TiltRange` (- _dmxchannel_maxvalue _dmxchannel_minvalue))
    (set `local.LocalPatch` (`DMXComponent.GetFixturePatch` (`DMXFixtureActor.DMX` _asbp_mover)))
    (if (`KismetArrayLibrary.Array_IsValidIndex` _returnvalue)
      (set `local.TiltPoint` (`|GetArrayItem` _returnvalue))
      (else
        (bind _returnvalue_2 (`AddComponent|NODE_AddSceneComponent-2` :`self` _movingheadref :`RelativeTransform` (`KismetMathLibrary.MakeTransform` (0.0 0.0 28.0))))
        (bind _output_get (set `local.TiltPoint` _returnvalue_2))
        (set `ActorComponent.ComponentTags` (`|MakeArray` "HeadTilt" :!type "Name") _output_get)
        (`SceneComponent.K2_AttachToComponent` _output_get _output "None" "KeepRelative" "KeepRelative" "KeepRelative" false)))
    (set `local.RotationPoint` _output)
    (`SceneComponent.K2_SetWorldRotation` _tiltpoint (`KismetMathLibrary.MakeRotFromXZ` (`SceneComponent.GetForwardVector` (`local.RotationPoint`)) (`KismetMathLibrary.Normal` (- (`self.K2_GetActorLocation`) (`SceneComponent.K2_GetComponentLocation` _tiltpoint)))) false false)
    (set `self.CurrentTiltAngle` 0.0)
    (`DMXSubsystem.SendDMX` (subsystem `DMXSubsystem`) (`local.LocalPatch`) (`|MakeMap` (struct :`Name` "Tilt") (`KismetMathLibrary.FTrunc` (* (- 1.0 (/ (+ (/ (`local.TiltRange`) 2.0) _relativerotation_roll) (`local.TiltRange`))) (select `EDMXFixtureSignalFormat` (`BlueprintMapLibrary.Map_Find` (`DMXEntityFixturePatch.GetAttributeSignalFormats` (`local.LocalPatch`)) (struct :`Name` "Tilt")) :`E8Bit` 255.0 :`E16Bit` 65536.0 :!type "Float (single-precision)"))) :!type "DMXAttributeName Structure"))
    (else
      (bind _asbp_mover_2 (cast `/Game/DMX/BP_Mover` object))
      (`SceneComponent.K2_SetRelativeRotation` :`self` (`/Game/DMX/BP_Mover.StaticMeshYoke` _asbp_mover_2)))))

(fn `UpdatePan`
  (params (object :type "Object Object Reference"))
  (locals (LocalPatch :type "DMXEntityFixturePatch Object Reference") (PanRange :type "Float (double-precision)") (MovingHeadRef :type "Actor Object Reference") (Yoke :type "StaticMeshComponent Object Reference") (RotationPoint :type "SceneComponent Object Reference") (Base :type "StaticMeshComponent Object Reference"))
  (bind _panrange (`local.PanRange`))
  (bind _rotationpoint (`local.RotationPoint`))
  (bind _returnvalue (`self.GetActorUpVector` (`local.MovingHeadRef`)))
  (bind _returnvalue_2 (`SceneComponent.GetRightVector` _rotationpoint))
  (bind _returnvalue_3 (`self.GetComponentsByTag` (`local.MovingHeadRef`) "/Script/Engine.SceneComponent" "YokeRot"))
  (bind (_relativerotation_roll _relativerotation_pitch _relativerotation_yaw) (`KismetMathLibrary.BreakRotator` (`SceneComponent.RelativeRotation` _rotationpoint)))
  (bind _returnvalue_4 (`KismetMathLibrary.Normal` (- (`self.K2_GetActorLocation`) (`SceneComponent.K2_GetComponentLocation` _rotationpoint))))
  (bind _returnvalue_5 (select `EDMXFixtureSignalFormat` (`BlueprintMapLibrary.Map_Find` (`DMXEntityFixturePatch.GetAttributeSignalFormats` (`local.LocalPatch`)) (struct :`Name` "Pan")) :`E8Bit` 255.0 :`E16Bit` 65536.0 :!type "Float (single-precision)"))
  (bind _returnvalue_6 (* _returnvalue_4 -1.0))
  (if (`self.bPan`)
    (bind _asbp_mover (cast `/Game/DMX/BP_Mover` object))
    (set `local.Base` (`/Game/DMX/BP_Mover.StaticMeshBase` _asbp_mover))
    (set `local.MovingHeadRef` _asbp_mover)
    (bind (_dmxchannel_minvalue _dmxchannel_maxvalue) (break `DMXChannelData` (`DMXFixtureComponentSingle.DMXChannel` (`/Game/DMX/BP_Mover.Pan_Component` _asbp_mover))))
    (set `local.PanRange` (- _dmxchannel_minvalue _dmxchannel_maxvalue))
    (set `local.LocalPatch` (`DMXComponent.GetFixturePatch` (`DMXFixtureActor.DMX` _asbp_mover)))
    (if (`KismetArrayLibrary.Array_IsValidIndex` _returnvalue_3)
      (set `local.RotationPoint` (`|GetArrayItem` _returnvalue_3))
      (else
        (bind _returnvalue_7 (`AddComponent|NODE_AddSceneComponent-1` :`self` (`local.MovingHeadRef`)))
        (bind _output_get (set `local.RotationPoint` _returnvalue_7))
        (set `ActorComponent.ComponentTags` (`|MakeArray` "YokeRot" :!type "Name") _output_get)
        (`SceneComponent.K2_AttachToComponent` _output_get (`local.Base`) "None" "SnapToTarget" "SnapToTarget" "SnapToTarget" false)))
    ;[1 1 1] YokeRotation
    (`SceneComponent.K2_SetWorldRotation` _rotationpoint (`KismetMathLibrary.SelectRotator` (`KismetMathLibrary.MakeRotFromZY` _returnvalue _returnvalue_4) (`KismetMathLibrary.MakeRotFromZY` _returnvalue _returnvalue_6) (> (`KismetMathLibrary.Dot_VectorVector` _returnvalue_2 _returnvalue_4) (`KismetMathLibrary.Dot_VectorVector` _returnvalue_2 _returnvalue_6))) false false)
    (bind _output_get_2 (set `self.CurrentPanAngle` (select `bool` (>= _relativerotation_yaw 0.0) :`false` (+ (- 180.0 (`KismetMathLibrary.Abs` _relativerotation_yaw)) 180.0) :`true` _relativerotation_yaw)))
    (`DMXSubsystem.SendDMX` (subsystem `DMXSubsystem`) (`local.LocalPatch`) (`|MakeMap` (struct :`Name` "Pan") (`KismetMathLibrary.FTrunc` (+ (* _returnvalue_5 (/ (/ (- _panrange 360.0) 2.0) _panrange)) (* (/ (`KismetMathLibrary.Abs` (- _output_get_2 (`KismetMathLibrary.SelectFloat` 360.0 0.0 (`self.FlipPanRotationDirection`)))) 360.0) (* _returnvalue_5 (/ 360.0 _panrange))))) :!type "DMXAttributeName Structure"))
    (else
      (bind _asbp_mover_2 (cast `/Game/DMX/BP_Mover` object))
      (`SceneComponent.K2_SetRelativeRotation` :`self` (`/Game/DMX/BP_Mover.StaticMeshYoke` _asbp_mover_2)))))

(fn `UpdateSelectedPatches`
  (if (`self.bUseTag`)
    (`self.GetAllFixturePatches` (`self.SearchTag`)))
  (for _array_element (`self.FixturePatch`)
    (`self.UpdatePan` _array_element)
    (`self.Update Tilt` _array_element)))

(fn `UserConstructionScript`
  (`self.UpdateSelectedPatches`))